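; GameplayCharacter is a playable character with standard jump, movement and look input, plus a replicated team identity.
; On the server, capsule hits from Slag actors launch the character along the negated, scaled impact normal with a fixed upward boost, and print a debug message.
; OnRep_Team swaps the mesh material to show red, blue or no team.
; An older Hit-based knockback variant remains unconnected.
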(event OnComponentHit(CapsuleComponent)
  (params (HitComponent :type Primitive%20Component%20Object%20Reference) (OtherActor :type Actor%20Object%20Reference) (OtherComp :type Primitive%20Component%20Object%20Reference) (NormalImpulse :type Vector :default "0, 0, 0") (Hit :type Hit%20Result%20Structure%20%28by%20ref%29))
  (bind _returnvalue (Math|Vector|Normalize NormalImpulse))
  (bind _returnvalue_2 (* _returnvalue -1e+03))
  (bind (_x _y) (Math|Vector|BreakVector _returnvalue_2))
  (Networking|SwitchHasAuthority
    (:Authority
      (Utilities|Casting|CastToSlag OtherActor)
      (Character|LaunchCharacter (Math|Vector|MakeVector _x _y 5e+02) false false)
      (Development|PrintString "Impulse added" true true "(R=0.000000,G=0.660000,B=1.000000,A=1.000000)" 2e+01))))

(event EventBeginPlay)

(event Collision|EventActorBeginOverlap
  (params (OtherActor :type Actor%20Object%20Reference)))

(event Game|Damage|EventPointDamage
  (params (Damage :type Float%20%28single-precision%29) (DamageType :type Damage%20Type%20Object%20Reference) (HitLocation :type Vector :default "0, 0, 0") (HitNormal :type Vector :default "0, 0, 0") (HitComponent :type Primitive%20Component%20Object%20Reference) (BoneName :type Name :default "None") (ShotFromDirection :type Vector :default "0, 0, 0") (InstigatedBy :type Controller%20Object%20Reference) (DamageCauser :type Actor%20Object%20Reference) (HitInfo :type Hit%20Result%20Structure%20%28by%20ref%29))
  ;[1 1 1] Damage Taken
)

(event EventTick
  (params (DeltaSeconds :type Float%20%28single-precision%29)))

(event Game|Damage|EventRadialDamage
  (params (DamageReceived :type Float%20%28single-precision%29) (DamageType :type Damage%20Type%20Object%20Reference) (Origin :type Vector :default "0, 0, 0") (HitInfo :type Hit%20Result%20Structure%20%28by%20ref%29) (InstigatedBy :type Controller%20Object%20Reference) (DamageCauser :type Actor%20Object%20Reference))
  ;[1 1 1] Damage Taken
)

(event Collision|EventHit
  (params (MyComp :type Primitive%20Component%20Object%20Reference) (Other :type Actor%20Object%20Reference) (OtherComp :type Primitive%20Component%20Object%20Reference) (bSelfMoved :type Boolean) (HitLocation :type Vector :default "0, 0, 0") (HitNormal :type Vector :default "0, 0, 0") (NormalImpulse :type Vector :default "0, 0, 0") (Hit :type Hit%20Result%20Structure%20%28by%20ref%29)))

(event Input|ActionEvents|InputActionJump
  (params (Key :type Key%20Structure))
  ;[1 1 1] Input
  (:Pressed
    (Character|Jump))
  (:Released
    (Character|StopJumping)))

(event Input|AxisEvents|InputAxisMoveRight
  (params (AxisValue :type Float%20%28single-precision%29))
  ;[1 1 1] Input
  (Pawn|Input|AddMovementInput (Transformation|GetActorRightVector) AxisValue false))

(event Input|AxisEvents|InputAxisMoveForward
  (params (AxisValue :type Float%20%28single-precision%29))
  ;[1 1 1] Input
  (Pawn|Input|AddMovementInput (Transformation|GetActorForwardVector) AxisValue false))

(event Input|AxisEvents|InputAxisLookUp
  (params (AxisValue :type Float%20%28single-precision%29))
  ;[1 1 1] Input
  (Pawn|Input|AddControllerPitchInput AxisValue))

(event Input|AxisEvents|InputAxisTurn
  (params (AxisValue :type Float%20%28single-precision%29))
  ;[1 1 1] Input
  (Pawn|Input|AddControllerYawInput AxisValue))

(fn ConstructionScript)

(fn OnRepTeam
  (bind _mesh (Variables|Character|GetMesh))
  (switch Utilities|FlowControl|Switch|SwitchonTeam (Variables|Default|GetTeam)
    (:NewEnumerator2
      (Rendering|Material|SetMaterial _mesh 0 "/Engine/Tutorial/SubEditors/TutorialAssets/Character/TutorialTPP_Mat.TutorialTPP_Mat"))
    (:NewEnumerator0
      (Rendering|Material|SetMaterial _mesh 0 "/Game/Materials/M_Red.M_Red"))
    (:NewEnumerator1
      (Rendering|Material|SetMaterial _mesh 0 "/Game/Materials/M_Blue.M_Blue"))))