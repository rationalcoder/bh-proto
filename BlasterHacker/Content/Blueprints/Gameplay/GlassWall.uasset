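; Destructible glass wall built as a Rows x Cols x Depth grid of instanced mesh chunks, spaced by mesh bounds in the construction script and stacked downward in Z.
; At BeginPlay it spawns a box-sized GlassCollider per chunk, tagged with its instance index and owning wall.
; On authority, DestroyGlassChunk has every GameplayGM controller call ClientDestroyChunk for that instance and wall type, then reports the damage to GameplayGM.
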(event Custom|DestroyGlassChunk
  (params (Collider :type Glass%20Collider%20Object%20Reference))
  (bind _self self)
  (bind _type (Variables|Default|GetType _self))
  (Networking|SwitchHasAuthority
    (:Authority
      (CallFunction|DestroyChunkonClients (Variables|/Game/Blueprints/Gameplay/GlassCollider.GlassCollider_C|GetTargetInstance Collider) _type)
      (bind _asgameplay_gm (Utilities|Casting|CastToGameplayGM (Game|GetGameMode)))
      (Default|WallDamaged _asgameplay_gm _type))))

(event EventBeginPlay
  (for (_array_element _array_index) (Variables|Default|GetTransforms)
    (bind _returnvalue (Game|SpawnActorfromClass "/Game/Blueprints/Gameplay/GlassCollider.GlassCollider_C" _array_element "AlwaysSpawn" 0 _array_index self 0))
    (Components|Box|SetBoxExtent (Variables|/Game/Blueprints/Gameplay/GlassCollider.GlassCollider_C|GetBox _returnvalue) (Math|Vector|MakeVector (/ (Variables|Default|GetDeltaX) 2.0) (/ (Variables|Default|GetDeltaY) 2.0) (/ (Variables|Default|GetDeltaZ) 2.0)) false)
    (Utilities|Array|Add (Variables|Default|GetColliders) _returnvalue)))

(fn ConstructionScript
  (bind _chunks (Variables|Default|GetChunks))
  (bind _chunks_2 (Variables|Default|GetChunks))
  (bind (_min _max) (Components|StaticMesh|GetLocalBounds _chunks))
  (bind (_x _y _z) (Math|Vector|BreakVector _max))
  (bind (_x_2 _y_2 _z_2) (Math|Vector|BreakVector _min))
  (Variables|Default|SetDeltaX (- _x _x_2))
  (Variables|Default|SetDeltaY (- _y _y_2))
  (Variables|Default|SetDeltaZ (- _z_2 _z))
  (for _index (range 0 (- (Variables|Default|GetRows) 1))
    (for _index_2 (range 0 (- (Variables|Default|GetCols) 1))
      (for _index_3 (range 0 (- (Variables|Default|GetDepth) 1))
        (bind _returnvalue (Components|InstancedStaticMesh|AddInstance _chunks_2 (Math|Transform|MakeTransform (Math|Vector|MakeVector (* _index_3 (Variables|Default|GetDeltaX)) (* _index_2 (Variables|Default|GetDeltaY)) (* _index (Variables|Default|GetDeltaZ))))))
        (Utilities|Array|Add (Variables|Default|GetTransforms) (.OutInstanceTransform (Components|InstancedStaticMesh|GetInstanceTransform _chunks_2 _returnvalue true))))))
  (Variables|Default|SetDeltaZ (Math|Float|Absolute(Float) (Variables|Default|GetDeltaZ))))

(fn DestroyChunkonClients
  (params (Instance :type Integer) (Wall :type WallType%20Enum :default "NewEnumerator0"))
  (bind _asgameplay_gm (Utilities|Casting|CastToGameplayGM (Game|GetGameMode)))
  (for _array_element (Variables|/Game/Blueprints/Gameplay/GameplayGM.GameplayGM_C|GetControllers _asgameplay_gm)
    (Default|ClientDestroyChunk _array_element Instance Wall)))