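; Game mode for a Red versus Blue match that spawns and respawns characters at random team-tagged player starts and ends when a team's wall is damaged.
; A countdown gates match start, then one-second timers periodically give every player slag and the same random item.
; It keeps a controller list to push timer updates, game-over results, sounds and effects, and to clean up before server travel to the lobby.
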(event Custom|Actual%20Add%20Custom%20Player
  (params (Team :type Team%20Enum :default "NewEnumerator2") (Player :type Gameplay%20PC%20Object%20Reference))
  ;[0 0 0] Player Starting
  (bind _start (CallFunction|ChooseCustomPlayerStart Team))
  (Default|ClientSetControllerRotation Player (.Rotation (Math|Transform|BreakTransform (Transformation|GetActorTransform _start))))
  (Default|SetTimerMaxes Player (Variables|Timing|GetMaxSlagSeconds) (Variables|Timing|GetMaxItemSeconds))
  (bind _returnvalue (Game|SpawnActorfromClass "/Game/Blueprints/Characters/GameplayCharacter.GameplayCharacter_C" (Transformation|GetActorTransform _start) "Undefined" Player 100 Team 0))
  (Pawn|Possess Player _returnvalue)
  (Variables|/Game/Blueprints/Characters/GameplayCharacter.GameplayCharacter_C|SetTeam _returnvalue Team)
  (Utilities|Array|Add (Variables|Default|GetControllers) Player))

(event Custom|CheckItemTimer
  (bind _controllers (Variables|Default|GetControllers))
  ;[0 0 0] Item Timing
  (if (== (Variables|Timing|GetItemSeconds) 0)
    (Variables|Timing|SetItemSeconds (Variables|Timing|GetMaxItemSeconds))
    (Variables|Timing|SetLocalRandomItem (Utilities|Enum|ByteToEnumItemType (Math|Conversions|ToByte(Integer) (Math|Random|RandomInteger (Math|Conversions|ToInteger(Byte) (Utilities|Enum|LiteralenumItemType "NewEnumerator3"))))))
    (for _array_element _controllers
      (Default|NewItem _array_element (Variables|Timing|GetLocalRandomItem)))
    (else
      (Math|Integer|DecrementInt (Variables|Timing|GetItemSeconds)
        (:%20%20
          _))))
  (for _array_element_2 _controllers
    (Default|UpdateItemTimer _array_element_2 (Variables|Timing|GetItemSeconds))))

(event Custom|Back%20To%20Lobby
  (for _array_element (Variables|Default|GetControllers)
    (Default|CleanupforTravel _array_element)
    (Development|ExecuteConsoleCommand "servertravel /Game/Maps/LobbyMap?FromGame=true")))

(event Custom|ItemTimerTick
  ;[0 0 0] Item Timing
  (if (not (Variables|Default|GetGameOver))
    (CallFunction|CheckItemTimer)
    (CallFunction|CheckSlagTimer)))

(event Custom|WaitTimerTick
  ;[0 0 0] Waiting for game to begin
  (for _array_element (Variables|Default|GetControllers)
    (Default|UpdateWaitTime _array_element (Variables|Timing|GetWaitSeconds)))
  (if (== (Variables|Timing|GetWaitSeconds) 0)
    (Utilities|Time|SetTimerbyEvent (delegate Custom|WaitTimerTick) 0.0)
    (else
      (Math|Integer|DecrementInt (Variables|Timing|GetWaitSeconds)))))

(event Custom|MulticastSpawnEffect
  (params (Location :type Vector) (Effect :type Particle%20System%20Object%20Reference))
  (for _array_element (Variables|Default|GetControllers)
    (Default|LocalSpawnEffect _array_element Effect Location)))

(event Custom|MulticastPlaySound
  (params (Location :type Vector) (Sound :type Sound%20Base%20Object%20Reference))
  (for _array_element (Variables|Default|GetControllers)
    (Default|LocalPlaySound _array_element Sound Location)))

(event Custom|CheckSlagTimer
  (bind _controllers (Variables|Default|GetControllers))
  ;[0 0 0] Item Timing
  (if (== (Variables|Timing|GetSlagSeconds) 0)
    (Variables|Timing|SetSlagSeconds (Variables|Timing|GetMaxSlagSeconds))
    (for _array_element _controllers
      (Default|AddSlag _array_element))
    (else
      (Math|Integer|DecrementInt (Variables|Timing|GetSlagSeconds)
        (:%20%20
          _))))
  (for _array_element_2 _controllers
    (Default|UpdateSlagTimer _array_element_2 (Variables|Timing|GetSlagSeconds))))

(event Custom|KillPlayer
  (params (Player :type Gameplay%20PC%20Object%20Reference) (Character :type Gameplay%20Character%20Object%20Reference))
  (CallFunction|KillPlayerFunction Player Character))

(event Custom|WallDamaged
  (params (Type :type WallType%20Enum :default "NewEnumerator0"))
  (bind _controllers (Variables|Default|GetControllers))
  ;[0 0 0] Game Over
  (if (not (Variables|Default|GetGameOver))
    (switch Utilities|FlowControl|Switch|SwitchonWallType Type
      (:NewEnumerator1
        (for _array_element _controllers
          (Default|GameOver _array_element "NewEnumerator1")
          (Utilities|Time|SetTimerbyEvent (delegate Custom|WaitTimerTick) 0.0)
          (Variables|Default|SetGameOver true)))
      (:NewEnumerator3
        (for _array_element_2 _controllers
          (Default|GameOver _array_element_2 "NewEnumerator0")
          (Utilities|Time|SetTimerbyEvent (delegate Custom|ItemTimerTick) 0.0)
          (Variables|Default|SetGameOver true))))))

(event EventHandleStartingNewPlayer
  (params (NewPlayer :type Player%20Controller%20Object%20Reference))
  ;[0 0 0] Player Starting
  (bind _asgameplay_pc (Utilities|Casting|CastToGameplayPC NewPlayer))
  (Default|GetCachedTeam _asgameplay_pc))

(event EventOnSetMatchState
  (params (NewState :type Name :default "None"))
  (if (Utilities|Name|Equal(Name) NewState "WaitingToStart")
    (Utilities|Time|SetTimerbyEvent (delegate Custom|WaitTimerTick) 1.0 true)
    (elif (Utilities|Name|Equal(Name) NewState "InProgress")
      (Utilities|Time|SetTimerbyEvent (delegate Custom|ItemTimerTick) 1.0 true))))

(fn ConstructionScript)

(fn RandomStart
  (params (Starts :type Array%20of%20Player%20Start%20Object%20References))
  (return (Utilities|Array|Get(acopy) Starts (Math|Random|RandomInteger (Utilities|Array|Length Starts)))))

(fn ChooseCustomPlayerStart
  (params (Team :type Team%20Enum :default "NewEnumerator2"))
  (if (Variables|Default|GetFirstTime)
    (CallFunction|FindPlayerStarts)
    (Variables|Default|SetFirstTime false))
  (switch Utilities|FlowControl|Switch|SwitchonTeam Team
    (:NewEnumerator2
      (return (stale _start) true))
    (:NewEnumerator0
      (bind _start (CallFunction|RandomStart (Variables|Default|GetRedStarts)))
      (return _start false))
    (:NewEnumerator1
      (bind _start_2 (CallFunction|RandomStart (Variables|Default|GetBlueStarts)))
      (return _start_2 false))))

(fn FindPlayerStarts
  (bind _outactors (Actor|GetAllActorsOfClass "/Script/Engine.PlayerStart"))
  (for _array_element _outactors
    (if (Utilities|Name|Equal(Name) (Variables|/Script/Engine.PlayerStart|GetPlayerStartTag _array_element) "Red")
      (Utilities|Array|Add (Variables|Default|GetRedStarts) _array_element)
      (else
        (Utilities|Array|Add (Variables|Default|GetBlueStarts) _array_element)))))

(fn KillPlayerFunction
  (params (Player :type Gameplay%20PC%20Object%20Reference) (Character :type Gameplay%20Character%20Object%20Reference))
  (LocalVariables|SetTeam (Variables|/Game/Blueprints/Characters/GameplayCharacter.GameplayCharacter_C|GetTeam Character))
  (bind _start (CallFunction|ChooseCustomPlayerStart (LocalVariables|GetTeam)))
  (Actor|DestroyActor Character)
  (bind _returnvalue (Game|SpawnActorfromClass "/Game/Blueprints/Characters/GameplayCharacter.GameplayCharacter_C" (Transformation|GetActorTransform _start) "Undefined" 0 100 (LocalVariables|GetTeam) 0))
  (Pawn|Possess Player _returnvalue)
  (Variables|/Game/Blueprints/Characters/GameplayCharacter.GameplayCharacter_C|SetTeam _returnvalue (LocalVariables|GetTeam)))

(fn ReadytoStartMatch
  (return (== (Variables|Timing|GetWaitSeconds) 0)))