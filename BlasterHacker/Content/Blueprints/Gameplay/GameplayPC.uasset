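; Gameplay player controller for a red-versus-blue team match, handling shooting, inventory, HUD updates and team handoff to GameplayGM.
; Input consumes slag ammo or the front of a five-slot item queue locally, then server events spawn impulse-launched projectiles.
; Server events also force or cancel the last item, apply radial damage and kill stuck players after a delay.
; Client chunk destruction removes glass wall instances, swapping the last collider into the freed index.
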(event Custom|GetCachedTeam
  (bind _asgame_info_instance (Utilities|Casting|CastToGameInfoInstance (Game|GetGameInstance)))
  (CallFunction|ServerGotCachedTeam (Variables|/Game/Blueprints/Common/GameInfoInstance.GameInfoInstance_C|GetCachedTeam _asgame_info_instance)))

(event Custom|ClientSetControllerRotation
  (params (Rotation :type Rotator))
  (Pawn|SetControlRotation Rotation))

(event Custom|Game%20Over
  (params (Winner :type Team%20Enum :default "NewEnumerator2"))
  ;[0 0 0] UI/Inventory
  (bind _asgameplay_hud (Utilities|Casting|CastToGameplayHUD (HUD|GetHUD)))
  (if (Utilities|Enum|Equal(Enum) Winner "NewEnumerator0")
    (Default|RedWins _asgameplay_hud)
    (else
      (Default|BlueWins _asgameplay_hud)))
  (if (Utilities|Enum|Equal(Enum) (Variables|Default|GetChosenTeam) Winner)
    (Audio|PlaySound2D "/Game/Sounds/Winner.Winner" 0.2)
    (else
      (Audio|PlaySound2D "/Game/Sounds/Loser.Loser" 0.2 2.0))))

(event Custom|Add%20Slag
  ;[0 0 0] UI/Inventory
  (bind _asgameplay_hud (Utilities|Casting|CastToGameplayHUD (HUD|GetHUD)))
  (Variables|Inventory|SetSlagCount 5)
  (Default|UpdateInventory _asgameplay_hud (Variables|Inventory|GetItems) (Variables|Inventory|GetSlagCount))
  (Audio|PlaySound2D "/Game/Sounds/SlagReload.SlagReload"))

(event Custom|ServerGotCachedTeam
  (params (Team :type Team%20Enum :default "NewEnumerator2"))
  (Variables|Default|SetChosenTeam Team)
  (bind _asgameplay_gm (Utilities|Casting|CastToGameplayGM (Game|GetGameMode)))
  (Default|ActualAddCustomPlayer _asgameplay_gm Team self))

(event Custom|SetInputModeGameOnly
  (Input|SetInputModeGameOnly self))

(event Custom|New%20Item
  (params (Item :type ItemType%20Enum :default "NewEnumerator1"))
  (bind _items (Variables|Inventory|GetItems))
  ;[0 0 0] UI/Inventory
  (bind _asgameplay_hud (Utilities|Casting|CastToGameplayHUD (HUD|GetHUD)))
  (Utilities|Array|Insert _items Item)
  (Utilities|Array|RemoveIndex _items 5)
  (Default|UpdateInventory _asgameplay_hud (Variables|Inventory|GetItems) (Variables|Inventory|GetSlagCount))
  (Audio|PlaySound2D "/Game/Sounds/ItemSound.ItemSound"))

(event Custom|ServerDeath
  (bind _self self)
  ;[0 0 0] Mid-Air Controls
  (bind _asgameplay_gm (Utilities|Casting|CastToGameplayGM (Game|GetGameMode)))
  (bind _asgameplay_character (Utilities|Casting|CastToGameplayCharacter (Pawn|GetControlledPawn _self)))
  (Default|KillPlayer _asgameplay_gm _self _asgameplay_character))

(event Custom|ServerDamageAtLocation
  (params (Location :type Vector))
  ;[0 0 0] Radial Damage Implementation. This must be done on the server.
  (Networking|SwitchHasAuthority
    (:Authority
      (Game|Damage|ApplyRadialDamage 1.0 Location 1e+03 0 0 (Pawn|GetControlledPawn) self true "ECC_Pawn")
      (Game|SpawnActorfromClass "/Game/Blueprints/Gameplay/Items/HackSphere.HackSphere_C" (Math|Transform|MakeTransform Location) "Undefined" 0 1e+02 0))))

(event Custom|Update%20Wait%20Time
  (params (SecondsLeft :type Integer))
  ;[0 0 0] UI/Inventory
  (bind _asgameplay_hud (Utilities|Casting|CastToGameplayHUD (HUD|GetHUD)))
  (Default|UpdateWaitTime _asgameplay_hud SecondsLeft))

(event Custom|Back%20To%20Lobby
  ;[0 0 0] UI/Inventory
  (bind _asgameplay_gm (Utilities|Casting|CastToGameplayGM (Game|GetGameMode)))
  (Default|BacktoLobby _asgameplay_gm))

(event Custom|ServerForceItem
  ;[0 0 0] Mid-Air Controls
  (Default|Force (Variables|Default|GetLastItem)))

(event Custom|Set%20Timer%20Maxes
  (params (Slag :type Integer) (Item :type Integer))
  ;[0 0 0] UI/Inventory
  (Variables|Default|SetSlagMax Slag)
  (Variables|Default|SetItemMax Item))

(event Custom|Update%20Item%20Timer
  (params (Seconds :type Integer))
  ;[0 0 0] UI/Inventory
  (bind _asgameplay_hud (Utilities|Casting|CastToGameplayHUD (HUD|GetHUD)))
  (Default|UpdateItemTime _asgameplay_hud Seconds (Variables|Default|GetItemMax)))

(event Custom|LocalSpawnEffect
  (params (Effect :type Particle%20System%20Object%20Reference) (Location :type Vector))
  (Effects|SpawnEmitteratLocation Effect Location "0, 0, 0" "2.000000,2.000000,2.000000"))

(event Custom|Update%20Slag%20Timer
  (params (Seconds :type Integer))
  ;[0 0 0] UI/Inventory
  (bind _asgameplay_hud (Utilities|Casting|CastToGameplayHUD (HUD|GetHUD)))
  (Default|UpdateSlagTime _asgameplay_hud Seconds (Variables|Default|GetSlagMax)))

(event Custom|ServerCancelItem
  ;[0 0 0] Mid-Air Controls
  (Actor|DestroyActor (Variables|Default|GetLastItem)))

(event Custom|Cleanup%20For%20Travel
  ;[0 0 0] UI/Inventory
  (Actor|DestroyActor (HUD|GetHUD))
  (Input|SetInputModeGameandUI 0 0 "DoNotLock" true))

(event Custom|ClientDestroyChunk
  (params (Instance :type Integer) (Wall :type WallType%20Enum :default "NewEnumerator0"))
  ;[0 0 0] Destroys Glass Chunk on Client
  (CallFunction|DestroyChunkinWall Instance Wall))

(event Custom|LocalPlaySound
  (params (Sound :type Sound%20Base%20Object%20Reference) (Location :type Vector))
  (Audio|PlaySoundatLocation Sound Location "0, 0, 0" 1.0 1.0 0.0 "/Game/Sounds/Attenuation.Attenuation"))

(event Custom|Use%20Slag
  ;[0 0 0] UI/Inventory
  (Math|Integer|DecrementInt (Variables|Inventory|GetSlagCount)
    (:%20%20
      (bind _asgameplay_hud (Utilities|Casting|CastToGameplayHUD (HUD|GetHUD)))
      (Default|UpdateInventory _asgameplay_hud (Variables|Inventory|GetItems) (Variables|Inventory|GetSlagCount)))))

(event Custom|Use%20Item
  (bind _items (Variables|Inventory|GetItems))
  ;[0 0 0] UI/Inventory
  (Utilities|Array|RemoveIndex _items)
  (Utilities|Array|Add _items "NewEnumerator4")
  (bind _asgameplay_hud (Utilities|Casting|CastToGameplayHUD (HUD|GetHUD)))
  (Default|UpdateInventory _asgameplay_hud _items (Variables|Inventory|GetSlagCount)))

(event Custom|ServerStuck
  ;[0 0 0] Mid-Air Controls
  (Utilities|Time|SetTimerbyEvent (delegate Custom|ServerDeath) 5.0))

(event Custom|ServerMulticastSound
  (params (Location :type Vector) (Sound :type Sound%20Base%20Object%20Reference))
  (bind _asgameplay_gm (Utilities|Casting|CastToGameplayGM (Game|GetGameMode)))
  (Default|MulticastPlaySound _asgameplay_gm Location Sound))

(event Custom|ServerShootItem
  (params (Item :type Base%20Item%20Class%20Reference) (Transform :type Transform) (ForwardVector :type Vector) (StartingVelocity :type Vector))
  ;[0 0 0] Common Item Shooting
  (Networking|SwitchHasAuthority
    (:Authority
      _)
    (:Remote
      _))
  (bind _returnvalue (Game|SpawnActorfromClass Item Transform "Undefined" 0 (Variables|Default|GetChosenTeam) 0 0))
  (Variables|/Game/Blueprints/Gameplay/Items/BaseItem.BaseItem_C|SetController _returnvalue self)
  (Transformation|SetActorScale3D _returnvalue "0.500000,0.500000,0.500000")
  (Physics|AddImpulse (Variables|/Game/Blueprints/Gameplay/Items/Slag.Slag_C|GetSphere _returnvalue) (+ ForwardVector (* ForwardVector 3e+03) StartingVelocity) "None" true)
  (if (!= Item "/Game/Blueprints/Gameplay/Items/Slag.Slag_C")
    (Variables|Default|SetLastItem _returnvalue)))

(event EventBeginPlay
  (CallFunction|SetInputModeGameOnly)
  (CallFunction|ClearInventory)
  (bind _outactors (Actor|GetAllActorsOfClass "/Game/Blueprints/Gameplay/GlassWall.GlassWall_C"))
  (for _array_element _outactors
    (switch Utilities|FlowControl|Switch|SwitchonWallType (Variables|/Game/Blueprints/Gameplay/GlassWall.GlassWall_C|GetType _array_element)
      (:NewEnumerator0
        (Variables|Default|SetRedGlass _array_element))
      (:NewEnumerator1
        (Variables|Default|SetRedWall _array_element))
      (:NewEnumerator2
        (Variables|Default|SetBlueGlass _array_element))
      (:NewEnumerator3
        (Variables|Default|SetBlueWall _array_element)))))

(event EventTick
  (params (DeltaSeconds :type Float%20%28single-precision%29)))

(event Input|ActionEvents|InputActionShootItem
  (params (Key :type Key%20Structure))
  ;[0 0 0] Item Shooting
  (:Pressed
    (bind _asgameplay_character (Utilities|Casting|CastToGameplayCharacter (Pawn|GetControlledPawn)))
    (switch Utilities|FlowControl|Switch|SwitchonItemType (Utilities|Array|Get(acopy) (Variables|Inventory|GetItems))
      (:NewEnumerator1
        (bind _output_get (Variables|Default|SetLocalShotItem "/Game/Blueprints/Gameplay/Items/ObstructionSpawner.ObstructionSpawner_C"))
        (CallFunction|UseItem)
        (CallFunction|ServerShootItem _output_get (Transformation|GetWorldTransform (Variables|/Game/Blueprints/Characters/GameplayCharacter.GameplayCharacter_C|GetShotTransform _asgameplay_character)) (Math|Vector|GetForwardVector (Variables|/Game/Blueprints/Characters/GameplayCharacter.GameplayCharacter_C|GetShotTransform _asgameplay_character)) "0, 0, 0"))
      (:NewEnumerator0
        (bind _output_get_2 (Variables|Default|SetLocalShotItem "/Game/Blueprints/Gameplay/Items/MissleSpawner.MissleSpawner_C"))
        (CallFunction|UseItem)
        (CallFunction|ServerShootItem _output_get_2 (Transformation|GetWorldTransform (Variables|/Game/Blueprints/Characters/GameplayCharacter.GameplayCharacter_C|GetShotTransform _asgameplay_character)) (Math|Vector|GetForwardVector (Variables|/Game/Blueprints/Characters/GameplayCharacter.GameplayCharacter_C|GetShotTransform _asgameplay_character)) "0, 0, 0"))
      (:NewEnumerator2
        (bind _output_get_3 (Variables|Default|SetLocalShotItem "/Game/Blueprints/Gameplay/Items/Orb.Orb_C"))
        (CallFunction|UseItem)
        (CallFunction|ServerShootItem _output_get_3 (Transformation|GetWorldTransform (Variables|/Game/Blueprints/Characters/GameplayCharacter.GameplayCharacter_C|GetShotTransform _asgameplay_character)) (Math|Vector|GetForwardVector (Variables|/Game/Blueprints/Characters/GameplayCharacter.GameplayCharacter_C|GetShotTransform _asgameplay_character)) (/ (Transformation|GetVelocity _asgameplay_character) 2.0))))))

(event Input|ActionEvents|InputActionShootSlag
  (params (Key :type Key%20Structure))
  ;[0 0 0] Item Shooting
  (:Pressed
    (bind _asgameplay_character (Utilities|Casting|CastToGameplayCharacter (Pawn|GetControlledPawn)))
    (if (> (Variables|Inventory|GetSlagCount) 0)
      (CallFunction|UseSlag)
      (CallFunction|ServerShootItem "/Game/Blueprints/Gameplay/Items/Slag.Slag_C" (Transformation|GetWorldTransform (Variables|/Game/Blueprints/Characters/GameplayCharacter.GameplayCharacter_C|GetShotTransform _asgameplay_character)) (Math|Vector|GetForwardVector (Variables|/Game/Blueprints/Characters/GameplayCharacter.GameplayCharacter_C|GetShotTransform _asgameplay_character)) (/ (Transformation|GetVelocity _asgameplay_character) 2.0)))))

(event Input|KeyboardEvents|F
  (params (Key :type Key%20Structure))
  ;[0 0 0] Mid-Air Controls
  (:Pressed
    (CallFunction|ServerForceItem)))

(event Input|KeyboardEvents|H
  (params (Key :type Key%20Structure))
  ;[0 0 0] Mid-Air Controls
  (:Pressed
    (CallFunction|ServerStuck)))

(event Input|KeyboardEvents|C
  (params (Key :type Key%20Structure))
  ;[0 0 0] Mid-Air Controls
  (:Pressed
    (CallFunction|ServerCancelItem)))

(fn ConstructionScript)

(fn DestroyChunkinWall
  (params (Instance :type Integer) (Wall :type WallType%20Enum :default "NewEnumerator0"))
  (switch Utilities|FlowControl|Switch|SwitchonWallType Wall
    (:NewEnumerator0
      (LocalVariables|SetTargetWall (Variables|Default|GetRedGlass)))
    (:NewEnumerator1
      (LocalVariables|SetTargetWall (Variables|Default|GetRedWall)))
    (:NewEnumerator2
      (LocalVariables|SetTargetWall (Variables|Default|GetBlueGlass)))
    (:NewEnumerator3
      (LocalVariables|SetTargetWall (Variables|Default|GetBlueWall))))
  (Class|InstancedStaticMeshComponent|RemoveInstance (Variables|/Game/Blueprints/Gameplay/GlassWall.GlassWall_C|GetChunks (LocalVariables|GetTargetWall)) Instance)
  (LocalVariables|SetColliderToDestroy (Utilities|Array|Get(acopy) (Variables|/Game/Blueprints/Gameplay/GlassWall.GlassWall_C|GetColliders (LocalVariables|GetTargetWall)) Instance))
  (bind _output_get (Variables|/Game/Blueprints/Gameplay/GlassCollider.GlassCollider_C|SetTargetInstance (Utilities|Array|Get(acopy) (Variables|/Game/Blueprints/Gameplay/GlassWall.GlassWall_C|GetColliders (LocalVariables|GetTargetWall)) (Utilities|Array|LastIndex (Variables|/Game/Blueprints/Gameplay/GlassWall.GlassWall_C|GetColliders (LocalVariables|GetTargetWall)))) Instance))
  (Utilities|Array|SetArrayElem (Variables|/Game/Blueprints/Gameplay/GlassWall.GlassWall_C|GetColliders (LocalVariables|GetTargetWall)) _output_get (Utilities|Array|Get(acopy) (Variables|/Game/Blueprints/Gameplay/GlassWall.GlassWall_C|GetColliders (LocalVariables|GetTargetWall)) (Utilities|Array|LastIndex (Variables|/Game/Blueprints/Gameplay/GlassWall.GlassWall_C|GetColliders (LocalVariables|GetTargetWall)))) true)
  (Utilities|Array|RemoveIndex (Variables|/Game/Blueprints/Gameplay/GlassWall.GlassWall_C|GetColliders (LocalVariables|GetTargetWall)) (Utilities|Array|LastIndex (Variables|/Game/Blueprints/Gameplay/GlassWall.GlassWall_C|GetColliders (LocalVariables|GetTargetWall))))
  (Actor|DestroyActor (LocalVariables|GetColliderToDestroy)))

(fn ClearInventory
  (bind _returnvalue (Utilities|Enum|LiteralenumItemType "NewEnumerator4"))
  (Variables|Inventory|SetItems (Utilities|Array|MakeArray _returnvalue _returnvalue _returnvalue _returnvalue _returnvalue))
  (Variables|Inventory|SetSlagCount 0))