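; Lobby game mode that registers joining players, spawns their characters at random player starts and launches the selected arena map.
; PostLogin initializes each LobbyPC from game instance and map settings, then possesses a fresh BasicCharacter.
; Server setting changes are pushed to every controller; each respawn rebroadcasts player info and recomputes CanStartGame from team choices.
; LaunchGame server-travels by map ID; kick-list and team-change events are empty stubs.
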(event Custom|ServerChangeTeam
  (params (Team :type Team%20Enum :default "NewEnumerator2") (PlayerController :type Player%20Controller%20Object%20Reference) (ChangedStatus :type Boolean)))

(event Custom|LaunchGame
  (bind _returnvalue (Game|GetPlayerController 0))
  ;[1 1 1] Launch game based on map selection from game settings.
  (switch int (Variables|State|GetGM_MapID)
    (:0
      (Development|ExecuteConsoleCommand "servertravel /Game/Maps/Arena01" _returnvalue))
    (:1
      (Development|ExecuteConsoleCommand "servertravel /Game/Maps/Arena2" _returnvalue))))

(event Custom|RespawnPlayer
  (params (Player :type Player%20Controller%20Object%20Reference))
  (bind _returnvalue (Pawn|GetControlledPawn Player))
  ;[1 1 1] Spawn players in the lobby, and tell everyone to update their lobbies with the latest information.
  (Utilities|IsValid _returnvalue
    (:Is%20Valid
      (Actor|DestroyActor _returnvalue))
    (:Is%20Not%20Valid
      _))
  (bind _start (CallFunction|ChooseCustomPlayerStart Player))
  (bind _returnvalue_2 (Game|SpawnActorfromClass "/Game/Blueprints/Characters/BasicCharacter.BasicCharacter_C" (Transformation|GetActorTransform _start) "AdjustIfPossibleButAlwaysSpawn" 0 100 0))
  (Pawn|Possess Player _returnvalue_2)
  (CallFunction|EveryoneUpdate))

(event Custom|AddToKickList)

(event Custom|ServerUpdateGameSettings
  (params (MapImage :type Texture%202D%20Object%20Reference) (MapName :type Text) (MapTime :type Text) (MapID :type Integer))
  ;[1 1 1] Server has made changes. Tell each client to update their lobby information.
  (Variables|State|SetGM_MapImage MapImage)
  (Variables|State|SetGM_MapName MapName)
  (Variables|State|SetGM_MapTime MapTime)
  (Variables|State|SetGM_MapID MapID)
  (for _array_element (Variables|State|GetAllPlayerControllers)
    (bind _aslobby_pc (Utilities|Casting|CastToLobbyPC _array_element))
    (Default|UpdateLobbySettings _aslobby_pc (Variables|State|GetGM_MapImage) (Variables|State|GetGM_MapName) (Variables|State|GetGM_MapTime))))

(event Custom|EveryoneUpdate
  (bind _allplayercontrollers (Variables|State|GetAllPlayerControllers))
  (bind _connectedplayerinformation (Variables|State|GetConnectedPlayerInformation))
  ;[1 1 1] Updated all connected player's lobby information.
  (bind _output_get (Variables|State|SetCurrentNumPlayers (Utilities|Array|Length (Variables|State|GetAllPlayerControllers))))
  (if (> _output_get 0)
    (Utilities|Array|Clear (Variables|State|GetConnectedPlayerInformation))
    (for _array_element _allplayercontrollers
      (bind _aslobby_pc (Utilities|Casting|CastToLobbyPC _array_element))
      (Utilities|Array|Add (Variables|State|GetConnectedPlayerInformation) (Variables|/Game/Blueprints/Lobby/LobbyPC.LobbyPC_C|GetPlayerSettings _aslobby_pc))
      (Default|UpdateNumberOfPlayers _aslobby_pc (Variables|State|GetCurrentNumPlayers) (Variables|State|GetMaxPlayers)))
    (for _array_element_2 _allplayercontrollers
      (bind _aslobby_pc_2 (Utilities|Casting|CastToLobbyPC _array_element_2))
      (Default|AddPlayerInfo _aslobby_pc_2 _connectedplayerinformation)
      (CallFunction|AddtoKickList))
    (Variables|State|SetCanStartGame true)
    (bind _array_element_3 (Utilities|Array|ForEachLoopwithBreak _connectedplayerinformation :!label _label)
      (:LoopBody
        (if (Utilities|Enum|Equal(Enum) (.Team (Utilities|Struct|BreakPlayerInfo _array_element_3)) "NewEnumerator2")
          (Variables|State|SetCanStartGame false)
          (goto _label Break))))))

(event EventPostLogin
  (params (NewPlayer :type Player%20Controller%20Object%20Reference))
  ;[1 1 1] Initial setup occurs on post login. This handles lobby setup for a new player controller and handles spawning.
  (Networking|SwitchHasAuthority
    (:Authority
      (Utilities|Array|Add (Variables|State|GetAllPlayerControllers) NewPlayer)
      (bind _outactors (Actor|GetAllActorsOfClass "/Script/Engine.PlayerStart"))
      (Variables|State|SetSpawnLocations _outactors)
      (bind _asgame_info_instance (Utilities|Casting|CastToGameInfoInstance (Game|GetGameInstance)))
      (Variables|State|SetServerName (Variables|/Game/Blueprints/Common/GameInfoInstance.GameInfoInstance_C|GetServerName _asgame_info_instance))
      (Variables|State|SetMaxPlayers (Variables|/Game/Blueprints/Common/GameInfoInstance.GameInfoInstance_C|GetMaxPlayers _asgame_info_instance))
      (bind _aslobby_pc (Utilities|Casting|CastToLobbyPC NewPlayer))
      (Default|InitialSetup _aslobby_pc)
      (Default|SetupLobbyMenu _aslobby_pc (Variables|State|GetServerName))
      (Default|UpdateLobbySettings _aslobby_pc (Variables|State|GetGM_MapImage) (Variables|State|GetGM_MapName) (Variables|State|GetGM_MapTime))
      (CallFunction|RespawnPlayer NewPlayer))))

(fn ConstructionScript)

(fn ChooseCustomPlayerStart
  (params (New%20Player :type Player%20Controller%20Object%20Reference))
  (bind _spawnlocations (Variables|State|GetSpawnLocations))
  (if (Math|Conversions|ToBoolean(Integer) (Utilities|Array|Length (Variables|State|GetSpawnLocations)))
    (Development|PrintString "choosing player start")
    (return (Utilities|Array|Get(acopy) _spawnlocations (Math|Random|RandomInteger (- (Utilities|Array|Length _spawnlocations) 1))))
    (else
      (Development|PrintString "Player Starts not initialized!!!"))))